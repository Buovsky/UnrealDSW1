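; Falling platform actor that dims its glow and drops after the third-person character steps into its trigger box.
; Overlap disables the box and plays an emissive fade timeline scaled to TimeToDisable, then enables physics on the floor after a short delay.
; Seconds later, ResetFloor stops physics, re-enables the box, restores the glow and moves the floor to the actor's saved start location, without resetting rotation.
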(event `self.ReceiveBeginPlay`
  (set `self.StartTransform` (`self.K2_GetActorLocation`)))

(event `self.Box.OnComponentBeginOverlap`
  (params (OverlappedComponent :type "PrimitiveComponent Object Reference") (OtherActor :type "Actor Object Reference") (OtherComp :type "PrimitiveComponent Object Reference") (OtherBodyIndex :type Integer) (bFromSweep :type Boolean) (SweepResult :type "HitResult Structure (by ref)"))
  (bind _floor (`self.Floor`))
  (cast `/Game/ThirdPerson/Blueprints/BP_ThirdPersonCharacter` OtherActor)
  (`PrimitiveComponent.SetCollisionEnabled` (`self.Box`) "NoCollision")
  (`TimelineComponent.SetPlayRate` (`self.EmissionFadeInOut`) (/ 1.0 (`self.TimeToDisable`)))
  (bind (_direction _fadeout) (`Timeline|EmissionFadeInOut` :`NewTime` 0.0 :!via `PlayFromStart`)
    (:`Update`
      (`MeshComponent.SetScalarParameterValueOnMaterials` (`self.Floor`) "EmissiveMultiplier" _fadeout))
    (:`Finished`
      (`KismetSystemLibrary.Delay` 0.2)
      (`MeshComponent.SetScalarParameterValueOnMaterials` _floor "EmissiveMultiplier" 0.0)
      (`PrimitiveComponent.SetSimulatePhysics` _floor true)
      (`KismetSystemLibrary.Delay` 5.0)
      (`self.ResetFloor`))))

(event `ResetFloor`
  (bind _floor (`self.Floor`))
  (`PrimitiveComponent.SetCollisionEnabled` (`self.Box`) "QueryAndPhysics")
  (`PrimitiveComponent.SetSimulatePhysics` _floor false)
  (`SceneComponent.K2_SetWorldLocation` _floor (`self.StartTransform`) false false)
  (`MeshComponent.SetScalarParameterValueOnMaterials` (`self.Floor`) "EmissiveMultiplier" 3.0))

(fn `UserConstructionScript`)